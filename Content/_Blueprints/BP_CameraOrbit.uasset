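; Orbit camera actor that becomes the view target, follows the BP_Bull and handles slingshot-style touch input to launch it.
; Tick snaps it to the bull and applies yaw while StartRotating is active.
; Touch drags become screen-relative pull values shown via BP_BullHUD; release calls ShootBull with camera forward and linear pull.
; The pull-driven rotation lerp is disconnected, and the mouse cursor is flagged for removal before shipping.
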(event EventTick
  (params (DeltaSeconds :type Float%20%28single-precision%29))
  (Utilities|FlowControl|Sequence
    (:then_0
      (if (Variables|Default|GetisRotating)
        (CallFunction|RotateOrbit)))
    (:then_1
      (Transformation|SetActorLocation (Transformation|GetActorLocation (Variables|Default|GetTarget)) false false))))

(event EventBeginPlay
  (Utilities|FlowControl|Sequence
    (:then_0
      (Variables|Default|SetstartRotation (Transformation|GetActorRotation))
      (bind _returnvalue (Actor|GetActorOfClass "/Game/_Blueprints/BP_Bull.BP_Bull_C"))
      (Variables|Default|SetTarget _returnvalue)
      (Game|Player|SetViewTargetwithBlend (Game|GetPlayerController 0) self (Variables|Default|GetblendTime) "VTBlend_Linear" 0.0 false))
    (:then_1
      ;[1 1 1] Initialize Widget
      (bind _returnvalue_2 (UserInterface|CreateWidget "/Game/_Blueprints/BP_BullHUD.BP_BullHUD_C"))
      (bind _output_get (Variables|Default|SetHUD _returnvalue_2))
      (UserInterface|Viewport|AddtoViewport _output_get 0))
    (:then_2
      ;[1 1 1] !REMOVE WHEN SHIPPING!
      (Variables|/Script/Engine.PlayerController|SetbShowMouseCursor (Game|GetPlayerController 0) true))))

(event Input|TouchEvents|InputTouch
  (params (Location :type Vector) (FingerIndex :type ETouchIndex%20Enum))
  (bind _returnvalue (Math|Conversions|ToVector2D(Vector) Location))
  (:Pressed
    ;[1 1 1] Initialize Pull
    (CallFunction|DetermineScreenResolution)
    (if (not (Variables|Default|GetwasShot))
      (Variables|Default|SetisPulling true)
      (Variables|Default|SetfingerStartPosition _returnvalue)
      (Default|ShowPullReference (Variables|Default|GetHUD) _returnvalue)
      (CallFunction|UpdateLinearPullForce _returnvalue)
      (CallFunction|UpdateAngularPullForce _returnvalue)))
  (:Released
    ;[1 1 1] End Pull
    (if (Variables|Default|GetisPulling)
      (Variables|Default|SetisPulling false)
      (Default|HidePullReference (Variables|Default|GetHUD))
      (if (> (Variables|Default|GetlinearPullVelocity) 0.0)
        (Default|ShootBull (Variables|Default|GetTarget) (Math|Vector|GetForwardVector (Transformation|GetWorldRotation (Variables|Default|GetRoot))) (Variables|Default|GetlinearPullVelocity)))))
  (:Moved
    ;[1 1 1] Process Pull
    (if (Variables|Default|GetisPulling)
      (CallFunction|UpdateLinearPullForce _returnvalue)
      (CallFunction|UpdateAngularPullForce _returnvalue))))

(fn ConstructionScript)

(fn RotateOrbit
  (bind _returnvalue (Transformation|GetActorRotation))
  (bind (_roll _pitch _yaw) (Math|Rotator|BreakRotator _returnvalue))
  (Transformation|SetActorRotation (Math|Rotator|MakeRotator _roll _pitch (+ _yaw (* (Math|Conversions|ToFloat(Integer) (Variables|Default|GetrotateDirection)) (Variables|Default|GetrotateSpeed))))))

(fn GetTargetRotation
  (if (Variables|Default|GetisPulling)
    (Development|PrintString (Utilities|String|ToString(Rotator) (Math|Rotator|MakeRotator (.Roll (Math|Rotator|BreakRotator (Variables|Default|GetstartRotation))) (+ (.Pitch (Math|Rotator|BreakRotator (Variables|Default|GetstartRotation))) (* (Variables|Default|GetlinearPullVelocity) (Variables|Default|GetmaximumYRotation))) (+ (.Yaw (Math|Rotator|BreakRotator (Variables|Default|GetstartRotation))) (* (Variables|Default|GetangularPullVelocity) (Variables|Default|GetmaximumZRotation))))))
    (return (Math|Rotator|MakeRotator (.Roll (Math|Rotator|BreakRotator (Variables|Default|GetstartRotation))) (+ (.Pitch (Math|Rotator|BreakRotator (Variables|Default|GetstartRotation))) (* (Variables|Default|GetlinearPullVelocity) (Variables|Default|GetmaximumYRotation))) (+ (.Yaw (Math|Rotator|BreakRotator (Variables|Default|GetstartRotation))) (* (Variables|Default|GetangularPullVelocity) (Variables|Default|GetmaximumZRotation)))))
    (else
      (bind _output_get (Variables|Default|SetstartRotation (Math|Rotator|MakeRotator (.Roll (Math|Rotator|BreakRotator (Variables|Default|GetstartRotation))) (.Pitch (Math|Rotator|BreakRotator (Variables|Default|GetstartRotation))) (.Yaw (Math|Rotator|BreakRotator (Transformation|GetWorldRotation (Variables|/Game/_Blueprints/BP_Bull.BP_Bull_C|GetBody (Variables|Default|GetTarget))))))))
      (return _output_get))))

(fn UpdateLinearPullForce
  (params (fingerPosition :type Vector%202D%20Structure))
  (bind _result (Math|Float|NegateFloat (.Y (Math|Vector2D|BreakVector2D (- (Variables|Default|GetfingerStartPosition) fingerPosition))))
    (:%20%20
      (Variables|Default|SetlinearPullVelocity (Math|Float|Clamp(Float) (/ (- _result (Variables|Default|GetpullVelocityThreshold)) (/ (.Y (Math|Vector2D|BreakVector2D (Variables|Default|GetscreenResolution))) 4.0)))))))

(fn UpdateAngularPullForce
  (params (fingerPosition :type Vector%202D%20Structure))
  (Variables|Default|SetangularPullVelocity (/ (.X (Math|Vector2D|BreakVector2D (- (Variables|Default|GetfingerStartPosition) fingerPosition))) (/ (.X (Math|Vector2D|BreakVector2D (Variables|Default|GetscreenResolution))) 2.0))))

(fn DetermineScreenResolution
  (bind _returnvalue (Game|GetPlayerController 0))
  (bind (_sizex _sizey) (HUD|GetViewportSize _returnvalue))
  (Variables|Default|SetscreenResolution (Math|Vector2D|MakeVector2D (Math|Conversions|ToFloat(Integer) _sizex) (Math|Conversions|ToFloat(Integer) _sizey))))

(fn StartRotating
  (params (RotateDirection :type Integer))
  (Variables|Default|SetrotateDirection RotateDirection)
  (Variables|Default|SetisRotating true))

(fn StopRotating
  (Variables|Default|SetrotateDirection 0)
  (Variables|Default|SetisRotating false))