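; BP_Bull is a physics-driven bull launched by an impulse scaled by pull strength.
; ShootBull turns the body red, lowers linear damping and starts a shot timer.
; Tick ends the shot once planar speed drops below a minimum after a brief delay, restoring blue material and heavy damping.
; Finger-pull and screen-resolution functions are unfinished, and the angular steering helpers are never called here.
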(event EventTick
  (params (DeltaSeconds :type Float%20%28single-precision%29))
  (if (Variables|Default|GetwasShot)
    (bind _shallkeepmoving (CallFunction|ShallStopMoving))
    (if _shallkeepmoving
      (Variables|Default|SetwasShot false)
      (Rendering|Material|SetMaterial (Variables|Default|GetBody) 0 (Variables|Default|GetblueMaterial))
      (else
        (Utilities|FlowControl|Sequence
          (:then_3
            (Variables|Default|SetdeltaTimeSinceShot (+ (Variables|Default|GetdeltaTimeSinceShot) (Utilities|Time|GetWorldDeltaSeconds)))))))
    (else
      (Class|PrimitiveComponent|SetLinearDamping (Variables|Default|GetBody) 1e+01))))

(fn ConstructionScript)

(fn UpdateLinearPullForce
  (params (fingerPosition :type Vector%202D%20Structure))
  (bind _result (Math|Float|NegateFloat (.Y (Math|Vector2D|BreakVector2D (- "" fingerPosition))))))

(fn UpdateAngularPullForce
  (params (fingerPosition :type Vector%202D%20Structure))
  (if (>= (.X (Math|Vector2D|BreakVector2D (- "" fingerPosition))) 0.0)
    _))

(fn ShootBull
  (params (forward :type Vector) (linearPullVelocity :type Float%20%28single-precision%29))
  (Physics|AddImpulse (Variables|Default|GetBody) (* forward (* (Variables|Default|GetlinearShootForce) linearPullVelocity)) "None" false)
  (Variables|Default|SetdeltaTimeSinceShot 0.0)
  (Variables|Default|SetwasShot true)
  (Rendering|Material|SetMaterial (Variables|Default|GetBody) 0 (Variables|Default|GetredMaterial))
  (Class|PrimitiveComponent|SetLinearDamping (Variables|Default|GetBody) 1.0))

(fn ShallStopMoving
  (return (and (>= (Variables|Default|GetminimumVelocity) (Math|Vector2D|Vector2DLength (Math|Conversions|ToVector2D(Vector) (Transformation|GetComponentVelocity (Variables|Default|GetBody))))) (>= (Variables|Default|GetdeltaTimeSinceShot) 0.1))))

(fn TransformAngulartoLinearVelocity
  (bind _body (Variables|Default|GetBody))
  (bind _returnvalue (Transformation|GetComponentVelocity _body))
  (bind _returnvalue_2 (Math|Conversions|ToVector2D(Vector) _returnvalue))
  (bind _returnvalue_3 (Math|Vector2D|Vector2DLength _returnvalue_2))
  (bind _returnvalue_4 (* "0, 0, 0" _returnvalue_3))
  (bind (_x _y) (Math|Vector|BreakVector _returnvalue_4))
  (Physics|SetPhysicsLinearVelocity _body (Math|Vector|MakeVector _x _y (.Z (Math|Vector|BreakVector _returnvalue))) false "None"))

(fn TurnThroughAngularVelocity
  (Class|PrimitiveComponent|SetPhysicsAngularVelocityinDegrees (Variables|Default|GetBody) (Math|Vector|MakeVector 0.0 0.0 (* 0.0 (Variables|Default|GetangularShootForce))) false "None"))

(fn DetermineScreenResolution)